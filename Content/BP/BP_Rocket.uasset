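; Player rocket character for an upgrade-and-launch game: climb to the finish distance to win, earning coins on failed runs.
; Loads saved stats and opens the shop; launching applies timeline-driven impulses, with the timeline chosen by MaxRunTime.
; A self-retriggering ToInfinity check tracks speed and distance, adjusts the camera arm and scrolls the star material for parallax.
; Reaching the finish shows the end screen; losing climb saves records and coinage, then shows game over.
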(event Custom|ReadyToLaunch
  ;[1 1 1] Ready to Launch
  (Audio|PlaySound2D "/Game/Sounds/Prepare4Launch/LaunchSound.LaunchSound" 1.0 1.0 0.0 0 0)
  (Widget|RemovefromParent (Variables|Default|GetAs%20UW%20Shop))
  (bind _returnvalue (UserInterface|CreateWidget "/Game/BP/UI/UW_Distance_Tracker.UW_Distance_Tracker_C"))
  (UserInterface|Viewport|AddtoViewport _returnvalue 0)
  (bind _returnvalue_2 (Actor|GetActorOfClass "/Game/BP/StartingPlatform.StartingPlatform_C"))
  (Variables|Default|SetAs%20Starting%20Platform _returnvalue_2)
  (Variables|/Script/Engine.PlayerController|SetbShowMouseCursor (Game|GetPlayerController 0) false)
  ;[1 1 1] Launch
  (bind _output_get (Variables|Default|SetReady2Launch true)))

(event Custom|To%20Infinity
  (bind _returnvalue (Transformation|GetVelocity))
  (bind _springarm (Variables|Default|GetSpringArm))
  (bind _returnvalue_2 (Math|Vector|VectorLength _returnvalue))
  ;[1 1 1] Set the spring arm length
  (Variables|Potential|SetPostitive%20or%20Negative (Math|Vector|DotProduct (Math|Vector|Normalize (Transformation|GetActorUpVector) 0.001) _returnvalue))
  (if (> (/ (+ _returnvalue_2 (Variables|/Script/Engine.SpringArmComponent|GetTargetArmLength _springarm)) 5e+02) 6e+02)
    (Variables|/Script/Engine.SpringArmComponent|SetTargetArmLength _springarm (Math|Float|Clamp(Float) (/ (+ _returnvalue_2 (Variables|/Script/Engine.SpringArmComponent|GetTargetArmLength _springarm)) 5e+02) 0.0 1e+04)))
  ;[1 1 1] Get the current speed
  (bind _output_get (Variables|Stats|SetCurrentSpeed (Math|Conversions|ToFloat(Integer) (Math|Float|Round (/ _returnvalue_2 1e+02)))))
  ;[1 1 1] Get the distance between Starting Platform and Spaceship
  (Variables|Default|SetParallax%20Offset (+ (* _output_get (/ (stale EventTick _output_get) -1e+03)) (Variables|Default|GetParallax%20Offset)))
  (if (> (Variables|Default|GetParallax%20Offset) 1.0)
    (Variables|Default|SetParallax%20Offset (.Remainder (Math|Float|Division(WholeandRemainder) (Variables|Default|GetParallax%20Offset) 1.0))))
  (CallFunction|UpdateParallaxScrolling (Variables|Default|GetParallax%20Offset))
  (Variables|Stats|SetDistanceTravelled (Math|Conversions|ToFloat(Integer) (Math|Float|Round (Math|Vector|VectorLength (- (Transformation|GetActorLocation (Variables|Default|GetAs%20Starting%20Platform)) (Transformation|GetActorLocation))))))
  (if (> (Variables|Stats|GetCurrentSpeed) (Variables|Stats|GetMaxSpeedAchieved))
    (Variables|Stats|SetMaxSpeedAchieved (Variables|Stats|GetCurrentSpeed)))
  (if (> (Variables|Stats|GetDistanceTravelled) (Variables|Stats|GetMaxDistance))
    (Variables|Stats|SetMaxDistance (Variables|Stats|GetDistanceTravelled)))
  (if (>= (/ (Variables|Stats|GetDistanceTravelled) 1e+02) (Variables|Default|GetFinishLine))
    (bind _returnvalue_3 (UserInterface|CreateWidget "/Game/BP/UI/UW_EndScreen.UW_EndScreen_C"))
    (UserInterface|Viewport|AddtoViewport _returnvalue_3 0)
    (Variables|/Script/Engine.PlayerController|SetbShowMouseCursor (Game|GetPlayerController 0) true :!label _label)
    (Game|SetGamePaused true)
    (elif (!= (<= (Variables|Potential|GetPostitive%20or%20Negative) 0.0) (AI|Components|NavMovement|IsMovingonGround (Variables|Character|GetCharacterMovement)))
      (CallFunction|SaveGame)
      (bind _returnvalue_4 (UserInterface|CreateWidget "/Game/BP/UI/UW_GameOverScreen.UW_GameOverScreen_C"))
      (UserInterface|Viewport|AddtoViewport _returnvalue_4 0)
      (goto _label)
      (else
        (Timeline|SlightDelay PlayFromStart
          (:Finished
            (CallFunction|ToInfinity)))))))

(event Custom|Update%20Parallax%20Scrolling
  (params (ParallaxSrolling :type Float%20%28double-precision%29))
  ;[1 1 1] UpdateTexCordinates
  (Rendering|Material|SetScalarParameterValueonMaterials (Variables|Default|GetBackground%20Stars) "InputOffsetLayer0" (* ParallaxSrolling 2.0)))

(event Input|EnhancedActionEvents|EnhancedInputActionIA_Launch
  (params (ActionValue :type Boolean) (ElapsedSeconds :type Float%20%28double-precision%29) (TriggeredSeconds :type Float%20%28double-precision%29) (InputAction :type Input%20Action%20Object%20Reference :default "/Game/BP/Inputs/IA_Launch.IA_Launch"))
  ;[1 1 1] Launch
  (:Triggered
    (if (and (stale Custom|ReadyToLaunch _output_get) (AI|Components|NavMovement|IsMovingonGround (Variables|Character|GetCharacterMovement)))
      (Variables|/Script/Engine.CharacterMovementComponent|SetMass (Variables|Character|GetCharacterMovement) (Variables|Upgradeables|GetMassOfShip))
      (if (== (Variables|Upgradeables|GetMaxRunTime) 5.0)
        (bind _upwards_movement (Timeline|LaunchSequence PlayFromStart)
          (:Update
            (Physics|AddImpulse (Variables|Character|GetCharacterMovement) (Math|Vector|MakeVector 0.0 0.0 (Math|Float|Lerp (Variables|Upgradeables|GetInitalThrust) (Variables|Upgradeables|GetTopSpeed) _upwards_movement)) true)
            (CallFunction|ToInfinity :!label _label)))
        (elif (== (Variables|Upgradeables|GetMaxRunTime) 1e+01)
          (bind _upwards_movement_2 (Timeline|Timeline PlayFromStart)
            (:Update
              (Physics|AddImpulse (Variables|Character|GetCharacterMovement) (Math|Vector|MakeVector 0.0 0.0 (Math|Float|Lerp (Variables|Upgradeables|GetInitalThrust) (Variables|Upgradeables|GetTopSpeed) _upwards_movement_2)) true)
              (goto _label)))
          (elif (== (Variables|Upgradeables|GetMaxRunTime) 15.0)
            (bind _upwards_movement_3 (Timeline|Timeline_0 PlayFromStart)
              (:Update
                (Physics|AddImpulse (Variables|Character|GetCharacterMovement) (Math|Vector|MakeVector 0.0 0.0 (Math|Float|Lerp (Variables|Upgradeables|GetInitalThrust) (Variables|Upgradeables|GetTopSpeed) _upwards_movement_3)) true)
                (goto _label)))
            (elif (== (Variables|Upgradeables|GetMaxRunTime) 2e+01)
              (bind _upwards_movement_4 (Timeline|Timeline_1 PlayFromStart)
                (:Update
                  (Physics|AddImpulse (Variables|Character|GetCharacterMovement) (Math|Vector|MakeVector 0.0 0.0 (Math|Float|Lerp (Variables|Upgradeables|GetInitalThrust) (Variables|Upgradeables|GetTopSpeed) _upwards_movement_4)) true)
                  (goto _label))))))))))

(event EventBeginPlay
  ;[1 1 1] Begin Play
  (Audio|PlaySound2D "/Game/Sounds/Background.Background" 1.0 1.0 0.0 0 0)
  (bind _returnvalue (SaveGame|DoesSaveGameExist "HomeInAFlash"))
  (if _returnvalue
    (bind _returnvalue_2 (SaveGame|LoadGamefromSlot "HomeInAFlash"))
    (bind _asbp_save (Utilities|Casting|CastToBP_Save _returnvalue_2))
    (Variables|Default|SetAs%20BP%20Save _asbp_save)
    (Variables|Upgradeables|SetTopSpeed (Variables|/Game/BP/SaveAndLoad/BP_Save.BP_Save_C|GetTopSpeed (Variables|Default|GetAs%20BP%20Save)))
    (Variables|Upgradeables|SetInitalThrust (Variables|/Game/BP/SaveAndLoad/BP_Save.BP_Save_C|GetInitalThrust (Variables|Default|GetAs%20BP%20Save)))
    (Variables|Upgradeables|SetMaxRunTime (Variables|/Game/BP/SaveAndLoad/BP_Save.BP_Save_C|GetMaxRunTime (Variables|Default|GetAs%20BP%20Save)))
    (Variables|Upgradeables|SetMassOfShip (Variables|/Game/BP/SaveAndLoad/BP_Save.BP_Save_C|GetMassOfShip (Variables|Default|GetAs%20BP%20Save)))
    (Variables|Stats|SetMaxSpeedAchieved (Variables|/Game/BP/SaveAndLoad/BP_Save.BP_Save_C|GetMaxSpeedAchieved (Variables|Default|GetAs%20BP%20Save)))
    (Variables|Stats|SetCoinage (Variables|/Game/BP/SaveAndLoad/BP_Save.BP_Save_C|GetCoinage (Variables|Default|GetAs%20BP%20Save)))
    (Variables|Stats|SetMaxDistance (Variables|/Game/BP/SaveAndLoad/BP_Save.BP_Save_C|GetMaxDistance (Variables|Default|GetAs%20BP%20Save)))
    (else
      (bind _returnvalue_3 (SaveGame|CreateSaveGameObject "/Game/BP/SaveAndLoad/BP_Save.BP_Save_C"))
      (Variables|/Game/BP/SaveAndLoad/BP_Save.BP_Save_C|SetCoinage _returnvalue_3 (Variables|Stats|GetCoinage))
      (Variables|/Game/BP/SaveAndLoad/BP_Save.BP_Save_C|SetInitalThrust _returnvalue_3 (Variables|Upgradeables|GetInitalThrust))
      (Variables|/Game/BP/SaveAndLoad/BP_Save.BP_Save_C|SetMassOfShip _returnvalue_3 (Variables|Upgradeables|GetMassOfShip))
      (Variables|/Game/BP/SaveAndLoad/BP_Save.BP_Save_C|SetMaxDistance _returnvalue_3 (Variables|Stats|GetMaxDistance))
      (Variables|/Game/BP/SaveAndLoad/BP_Save.BP_Save_C|SetMaxSpeedAchieved _returnvalue_3 (Variables|Stats|GetMaxSpeedAchieved))
      (Variables|/Game/BP/SaveAndLoad/BP_Save.BP_Save_C|SetMaxRunTime _returnvalue_3 (Variables|Upgradeables|GetMaxRunTime))
      (Variables|/Game/BP/SaveAndLoad/BP_Save.BP_Save_C|SetTopSpeed _returnvalue_3 (Variables|Upgradeables|GetTopSpeed))
      (SaveGame|SaveGametoSlot _returnvalue_3 "HomeInAFlash")
      (Variables|Default|SetAs%20BP%20Save _returnvalue_3)))
  (bind _asplayer_controller (Utilities|Casting|CastToPlayerController (Pawn|GetController)))
  (Input|AddMappingContext (PlayerController|LocalPlayerSubsystems|GetEnhancedInputLocalPlayerSubsystem _asplayer_controller) "/Game/BP/Inputs/InputMapping.InputMapping" 0 "(bIgnoreAllPressedKeysUntilRelease=True,bForceImmediately=False)")
  (Variables|Default|SetReady2Launch false)
  (bind _returnvalue_4 (UserInterface|CreateWidget "/Game/BP/UI/UW_Shop.UW_Shop_C"))
  (bind _output_get (Variables|Default|SetAs%20UW%20Shop _returnvalue_4))
  (UserInterface|Viewport|AddtoViewport _returnvalue_4 0)
  (Variables|/Script/Engine.PlayerController|SetbShowMouseCursor (Game|GetPlayerController 0) true))

(event EventTick
  (params (DeltaSeconds :type Float%20%28single-precision%29))
  ;[1 1 1] Get the current speed
  (bind _output_get (Variables|Default|SetDelta%20Seconds DeltaSeconds)))

(fn ConstructionScript)

(fn SaveGame
  (bind _as_bp_save (Variables|Default|GetAs%20BP%20Save))
  (bind _as_bp_save_2 (Variables|Default|GetAs%20BP%20Save))
  (bind _distancetravelled (Variables|Stats|GetDistanceTravelled))
  (bind _returnvalue (/ _distancetravelled 200))
  (bind _returnvalue_2 (SaveGame|DoesSaveGameExist "HomeInAFlash"))
  (if _returnvalue_2
    (if (> (Variables|Stats|GetMaxSpeedAchieved) (Variables|/Game/BP/SaveAndLoad/BP_Save.BP_Save_C|GetMaxSpeedAchieved _as_bp_save))
      (Variables|/Game/BP/SaveAndLoad/BP_Save.BP_Save_C|SetMaxSpeedAchieved _as_bp_save (Variables|Stats|GetMaxSpeedAchieved)))
    (if (> (Variables|Stats|GetMaxDistance) (Variables|/Game/BP/SaveAndLoad/BP_Save.BP_Save_C|GetMaxDistance _as_bp_save))
      (Variables|/Game/BP/SaveAndLoad/BP_Save.BP_Save_C|SetMaxDistance _as_bp_save (Variables|Stats|GetMaxDistance)))
    (Variables|Default|SetCoinageDifference (Math|Conversions|ToFloat(Integer) _returnvalue))
    (bind _output_get (Variables|Stats|SetCoinage (+ (Variables|Stats|GetCoinage) _returnvalue)))
    (Variables|/Game/BP/SaveAndLoad/BP_Save.BP_Save_C|SetCoinage _as_bp_save_2 _output_get)
    (Variables|/Game/BP/SaveAndLoad/BP_Save.BP_Save_C|SetInitalThrust _as_bp_save_2 (Variables|Upgradeables|GetInitalThrust))
    (Variables|/Game/BP/SaveAndLoad/BP_Save.BP_Save_C|SetMassOfShip _as_bp_save_2 (Variables|Upgradeables|GetMassOfShip))
    (Variables|/Game/BP/SaveAndLoad/BP_Save.BP_Save_C|SetMaxRunTime _as_bp_save_2 (Variables|Upgradeables|GetMaxRunTime))
    (Variables|/Game/BP/SaveAndLoad/BP_Save.BP_Save_C|SetTopSpeed _as_bp_save_2 (Variables|Upgradeables|GetTopSpeed))
    (SaveGame|SaveGametoSlot (Variables|Default|GetAs%20BP%20Save) "HomeInAFlash")))